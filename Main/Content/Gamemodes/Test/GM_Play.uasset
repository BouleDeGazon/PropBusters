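; GM_Play is a test game mode that splits players into Busters and Ghasts.
; Two seconds after BeginPlay, it calls a multicast event that loops over every BP_Player and sets its role through ServerSetPlayer, passing its mesh and PropPlayer.
; Players become Busters until BustersTotal reaches half the player count, then the rest become Ghasts.
; The random indices stored in BustersTotal only serve as a count, so actor order decides roles.
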(event Custom|Multicast_SpawnPlayers
  ;[1 1 1] Set Player as Buster or Ghast
  (bind _outactors (Actor|GetAllActorsOfClass "/Game/Characters/BP_Player.BP_Player_C"))
  (bind _array_element (Utilities|Array|ForEachLoopwithBreak _outactors)
    (:LoopBody
      (if (== (Utilities|Array|Length (Variables|Default|GetBustersTotal)) (/ (Utilities|Array|Length _outactors) 2))
        (Default|ServerSetPlayer _array_element false (Variables|/Script/Engine.Character|GetMesh _array_element) (Variables|/Game/Characters/BP_Player.BP_Player_C|GetPropPlayer _array_element))
        (else
          (Default|ServerSetPlayer _array_element true (Variables|/Script/Engine.Character|GetMesh _array_element) (Variables|/Game/Characters/BP_Player.BP_Player_C|GetPropPlayer _array_element))
          (Utilities|Array|Add (Variables|Default|GetBustersTotal) (Math|Random|RandomIntegerinRange 0 (- (Utilities|Array|Length _outactors) 1))))))))

(event EventBeginPlay
  (Utilities|FlowControl|Delay 2.0)
  (CallFunction|MulticastSpawnPlayers))

(fn ConstructionScript)