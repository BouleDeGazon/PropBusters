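; Player character for a Buster-or-Ghast prop game, with server events for role, rotation, interaction, health and death.
; Tick turns the mesh toward screen-rotated input, sphere-traces for interactables (StartTrace's outline highlight is disconnected), runs the game-over countdown and checks death.
; Interact lets Busters pick up or throw BP_fuck props, each throw costing the thrower health.
; Interact also line-traces ahead to copy a hit object's skeletal mesh, regardless of role.
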(event Custom|Server_SetPlayer
  (params (IsBuster :type Boolean) (CharacterMesh0 :type Skeletal%20Mesh%20Component%20Object%20Reference) (PropPlayer :type Static%20Mesh%20Component%20Object%20Reference))
  ;[1 1 1] Set Player Buster or Ghast
  (bind _output_get (Variables|Default|SetIs%20Buster IsBuster))
  (if _output_get
    (Rendering|SetVisibility PropPlayer false false)
    (Collision|SetCollisionEnabled PropPlayer "NoCollision")
    (else
      (Rendering|SetVisibility CharacterMesh0 false false)
      (Collision|SetCollisionEnabled CharacterMesh0 "NoCollision"))))

(event Custom|PlayerDeath_Server
  ;[1 1 1] Global Functions
  ;;[1 1 1] Player Death
  (Actor|DestroyActor)
  (CallFunction|PlayerDeathMulticast))

(event Custom|HealthLoss_Multicast
  (params (PlayerHealth :type Integer))
  ;[1 1 1] Global Functions
  ;;[1 1 1] Player Damage
  (bind _output_get (Variables|Default|SetPlayerHealth PlayerHealth))
  (Development|PrintString (Utilities|String|ToString(Integer) _output_get)))

(event Custom|HealthLoss_Server
  (params (PlayerHealth :type Integer))
  ;[1 1 1] Global Functions
  ;;[1 1 1] Player Damage
  (bind _output_get (Variables|Default|SetPlayerHealth PlayerHealth))
  (CallFunction|HealthLossMulticast _output_get))

(event Custom|PropInteraction_Replicate_Server
  ;[1 1 1] Calls
  (CallFunction|PropInteraction))

(event Custom|PlayerDeath_Multicast
  ;[1 1 1] Global Functions
  ;;[1 1 1] Player Death
  (Actor|DestroyActor))

(event Custom|PlayerRotation_Replicate_Server
  (params (PlayerMesh :type Scene%20Component%20Object%20Reference) (RelativeRotation :type Rotator))
  ;[1 1 1] Global Functions
  ;;[1 1 1] Player Movement
  ;;;[1 1 1] Player Rotation
  ;;;;[1 1 1] Server Replication
  (Transformation|SetWorldRotation PlayerMesh RelativeRotation false false))

(event EventTick
  (params (DeltaSeconds :type Float%20%28single-precision%29))
  (bind _returnvalue (Input|AxisValues|GetUpDown))
  (bind _returnvalue_2 (Input|AxisValues|GetLeftRight))
  (bind _mesh (Variables|Character|GetMesh))
  (bind _mesh_2 (Variables|Character|GetMesh))
  (bind _returnvalue_3 (Transformation|GetWorldLocation _mesh_2))
  ;[1 1 1] Inputs
  (Utilities|FlowControl|Sequence
    (:then_0
      ;[1 1 1] Global Functions
      ;;[1 1 1] Player Movement
      ;;;[1 1 1] Player Rotation
      ;;;;[1 1 1] Using input as direction + Rotating axis to screen space
      (if (or (!= _returnvalue 0.0) (!= _returnvalue_2 0.0))
        (Variables|Default|SetPlayerDirection (Math|Vector|MakeVector (+ _returnvalue _returnvalue_2) (- _returnvalue_2 _returnvalue) 0.0))
        (CallFunction|PlayerRotationReplicateServer _mesh (Math|Rotator|Lerp(Rotator) (Transformation|GetWorldRotation _mesh) (Math|Conversions|RotationFromXVector (Variables|Default|GetPlayerDirection)) (* DeltaSeconds (Variables|Default|GetRotationSpeed)) true))))
    (:then_1
      ;[1 1 1] MEF
      (bind (_outhit _returnvalue_4) (Collision|SphereTraceForObjects _returnvalue_3 (+ (* (Math|Vector|GetForwardVector (Transformation|GetWorldRotation _mesh_2)) (Variables|Default|GetReach)) _returnvalue_3) (Variables|Default|GetRadius) (Utilities|Array|MakeArray "ObjectTypeQuery7") false 0 "ForOneFrame"))
      (if _returnvalue_4
        (if (== (.hitactor (Variables|Default|GetcanInteract)) (.HitActor (Collision|BreakHitResult _outhit)))
          (Variables|Default|SetcanInteract _outhit)
          (Utilities|FlowControl|DoOnce false :!label _label
            (:Completed
              (CallFunction|StopTrace)))
          (else
            (CallFunction|StartTrace (.HitActor (Collision|BreakHitResult _outhit)) (.hitactor (Variables|Default|GetcanInteract)))))
        (else
          (goto _label))))
    (:then_2
      ;[1 1 1] Countdown Timer
      (Utilities|FlowControl|Delay 1.0)
      (if (== (Variables|Default|GetSeconds) 0)
        (if (== (Variables|Default|GetMinutes) 0)
          (bind _returnvalue_5 (UserInterface|CreateWidget "/Game/UI/test/UI_GameOver.UI_GameOver_C"))
          (UserInterface|Viewport|AddtoViewport _returnvalue_5 0)
          (Variables|/Script/Engine.PlayerController|SetbShowMouseCursor (Game|GetPlayerController 0) true)
          (Game|SetGamePaused true)
          (else
            (Variables|Default|SetSeconds 59)
            (Variables|Default|SetMinutes (- (Variables|Default|GetMinutes) 1))))
        (else
          (Variables|Default|SetSeconds (- (Variables|Default|GetSeconds) 1)))))
    (:then_3
      ;;[1 1 1] Player Death
      (if (<= (Variables|Default|GetPlayerHealth) 0)
        (Actor|DestroyActor)
        (CallFunction|PlayerDeathServer)))))

(event Input|ActionEvents|InputActionInteract
  (params (Key :type Key%20Structure :default "None"))
  (bind _mesh (Variables|Character|GetMesh))
  (bind _returnvalue (Transformation|GetWorldLocation _mesh))
  ;[1 1 1] Inputs
  (:Pressed
    (Utilities|FlowControl|Sequence
      (:then_0
        ;[1 1 1] Calls
        (if (Variables|Default|GetIs%20Buster)
          (CallFunction|PropInteractionReplicateServer)))
      (:then_1
        ;[1 1 1] Detect in player radius
        (bind (_outhit _returnvalue_2) (Collision|LineTraceByChannel _returnvalue (+ _returnvalue (* (Math|Vector|GetForwardVector _mesh) 5e+03)) "TraceTypeQuery1" false 0 "ForOneFrame"))
        (if _returnvalue_2
          (bind _ascapsule_collision (Utilities|Casting|CastToCapsuleComponent (.HitComponent (Collision|BreakHitResult _outhit))))
          (bind _asskeletal_mesh_component (Utilities|Casting|CastToSkeletalMeshComponent (Components|GetChildComponent _ascapsule_collision 0)))
          (Class|SkinnedMeshComponent|SetSkeletalMesh (Variables|Character|GetMesh) (Variables|/Script/Engine.SkinnedMeshComponent|GetSkeletalMesh _asskeletal_mesh_component) true))))))

(event Input|AxisEvents|InputAxisUpDown
  (params (AxisValue :type Float%20%28single-precision%29))
  ;[1 1 1] Inputs
  ;[1 1 1] Global Functions
  ;;[1 1 1] Player Movement
  ;;;[1 1 1] Player Translation
  (Pawn|Input|AddMovementInput (* (Variables|Default|GetUpDownSpeed) (Variables|Default|GetMovementSpeed)) AxisValue false))

(event Input|AxisEvents|InputAxisLeftRight
  (params (AxisValue :type Float%20%28single-precision%29))
  ;[1 1 1] Inputs
  ;[1 1 1] Global Functions
  ;;[1 1 1] Player Movement
  ;;;[1 1 1] Player Translation
  (Pawn|Input|AddMovementInput (* (Variables|Default|GetLeftRightSpeed) (Variables|Default|GetMovementSpeed)) AxisValue false))

(fn ConstructionScript)

(fn StartTrace
  (params (newActor :type Actor%20Object%20Reference) (oldActor :type Actor%20Object%20Reference)))

(fn StopTrace
  (Utilities|FlowControl|Sequence
    (:then_0
      (if (not (== (.hitactor (Variables|Default|GetcanInteract)) 0))
        (Rendering|SetRenderCustomDepth (Utilities|Array|Get(acopy) (Actor|GetComponentsbyTag (.hitactor (Variables|Default|GetcanInteract)) "/Script/Engine.PrimitiveComponent" "outline")) false)))
    (:then_1
      (Variables|Default|SetcanInteract ""))))

(fn PropInteraction
  (bind _mesh (Variables|Character|GetMesh))
  (bind _propholdinglocation (Variables|Default|GetPropHoldingLocation))
  (bind _returnvalue (Transformation|GetWorldLocation _mesh))
  ;[1 1 1] Buster Functions
  ;;[1 1 1] Prop Throw
  (Utilities|IsValid (Variables|Default|GetHoldingProp)
    (:Is%20Valid
      (Development|PrintString "Player is already holding prop!")
      (Transformation|DetachFromComponent (Variables|/Script/Engine.Actor|GetRootComponent (Variables|Default|GetHoldingProp)) "KeepWorld" "KeepWorld" "KeepWorld" true)
      (bind _asbp_fuck (Utilities|Casting|CastToBP_fuck (Variables|Default|GetHoldingProp)))
      (Transformation|AttachComponentToComponent (Variables|/Game/Assets/BP_fuck.BP_fuck_C|GetPropSkeletalMesh _asbp_fuck) (Variables|/Script/Engine.Actor|GetRootComponent _asbp_fuck) "None" "SnapToTarget" "SnapToTarget" "KeepWorld" true)
      (Collision|SetCollisionEnabled (Variables|/Game/Assets/BP_fuck.BP_fuck_C|GetPropSkeletalMesh _asbp_fuck) "QueryAndPhysics")
      (Physics|AddImpulse (Variables|/Game/Assets/BP_fuck.BP_fuck_C|GetPropSkeletalMesh _asbp_fuck) (* (+ (Math|Vector|GetForwardVector (Variables|Character|GetMesh)) "1.000000,0.000000,0.000000") (Variables|Default|GetThrowingForce)) "None" true)
      (Development|PrintString "PROPTHROWN")
      (Variables|Default|SetHoldingProp 0)
      ;;;[1 1 1] Substract From Health
      (bind _output_get (Variables|Default|SetPlayerHealth (- (Variables|Default|GetPlayerHealth) 5)))
      (CallFunction|HealthLossServer _output_get))
    (:Is%20Not%20Valid
      ;;[1 1 1] Prop Pickup
      ;;;[1 1 1] Detect in player radius
      (bind (_outhit _returnvalue_2) (Collision|LineTraceForObjects _returnvalue (+ _returnvalue (* (* (Math|Vector|GetForwardVector (Transformation|GetWorldRotation _mesh)) (Variables|Default|GetReach)) (Variables|Default|GetRadius))) (Utilities|Array|MakeArray "ObjectTypeQuery7") false 0 "None"))
      (if _returnvalue_2
        (bind _asbp_fuck_2 (Utilities|Casting|CastToBP_fuck (.HitActor (Collision|BreakHitResult _outhit))))
        (Utilities|IsValid (Variables|Default|GetHoldingProp)
          (:Is%20Not%20Valid
            ;;;[1 1 1] Disable collisions & gravity on prop
            (Collision|SetCollisionEnabled (Variables|/Game/Assets/BP_fuck.BP_fuck_C|GetPropSkeletalMesh _asbp_fuck_2) "NoCollision")
            ;;;[1 1 1] Snap to player's head
            (Variables|Default|SetHoldingProp _asbp_fuck_2)
            (Transformation|AttachComponentToComponent _asbp_fuck_2 _propholdinglocation "None" "SnapToTarget" "SnapToTarget" "KeepWorld" true)
            (Transformation|AttachComponentToComponent (Variables|/Game/Assets/BP_fuck.BP_fuck_C|GetPropSkeletalMesh _asbp_fuck_2) _propholdinglocation "None" "SnapToTarget" "SnapToTarget" "KeepWorld" true)
            (Development|PrintString "Player is holding prop")))
        (else
          (Development|PrintString "No prop to grab!"))))))

(fn OnRepPlayerRotation)