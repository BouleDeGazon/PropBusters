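; GM_Play is a test game mode that randomly assigns players the Buster or Ghast role.
; Two seconds after BeginPlay it calls a multicast event that gathers all BP_Player actors and picks one random index as the Buster.
; It then calls ServerSetPlayer on each actor, marking the chosen one as Buster and the rest as Ghasts.
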(event Custom|Multicast_SpawnPlayers
  ;[1 1 1] Is Player Buster or Ghast?
  (bind _outactors (Actor|GetAllActorsOfClass "/Game/Characters/BP_Player.BP_Player_C"))
  (Variables|Default|SetBusterID (Math|Random|RandomIntegerinRange 0 (- (Utilities|Array|Length _outactors) 1)))
  (for (_array_element _array_index) _outactors
    (if (== _array_index (Variables|Default|GetBusterID))
      (Default|ServerSetPlayer _array_element true (Variables|/Game/Characters/BP_Player.BP_Player_C|GetBusterPlayer _array_element) (Variables|/Game/Characters/BP_Player.BP_Player_C|GetGhastPlayer _array_element))
      (else
        (Default|ServerSetPlayer _array_element false (Variables|/Game/Characters/BP_Player.BP_Player_C|GetBusterPlayer _array_element) (Variables|/Game/Characters/BP_Player.BP_Player_C|GetGhastPlayer _array_element))))))

(event EventBeginPlay
  ;[1 1 1] Is Player Buster or Ghast?
  (Utilities|FlowControl|Delay 2.0)
  (CallFunction|MulticastSpawnPlayers))

(fn ConstructionScript)